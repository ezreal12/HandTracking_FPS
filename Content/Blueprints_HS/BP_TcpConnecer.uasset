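; TCP client that connects to a local server and turns its messages into first-person character controls.
; Each slash-delimited message yields four directional values and an event code.
; The directions merge into signed X/Y, pass a dead-zone filter and drive MoveCamera, with X mirrored for a user-facing camera.
; The event code triggers weapon fire, flight or both, and a falling fallback ends flight when the flight code is absent.
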(event `self.ReceiveBeginPlay`
  ;[1 1 1] 시작시 기본값 설정j
  (set `self.compensateVal` 3.0)
  (`self.Connect` "127.0.0.1" 8888 (delegate `OnDis`) (delegate `OnConn`) (delegate `ReciveMsg`))
  (bind _asbp_first_person_character (cast `/Game/Blueprints_HS/BP_FirstPersonCharacter` (`GameplayStatics.GetPlayerPawn` 0))
    (:`then`
      (`KismetSystemLibrary.PrintString` "Casting OK")
      (set `self.As BP First Person Character` _asbp_first_person_character))
    (:`CastFailed`
      (`KismetSystemLibrary.PrintString` "Fail"))))

(event `OnDis`
  (params (ConnectionId :type Integer))
  (`KismetSystemLibrary.PrintString` "DisConnected"))

(event `OnConn`
  (params (ConnectionId :type Integer))
  (bind _output_get (set `self.sendMSG` "On Connected"))
  (`KismetSystemLibrary.PrintString` _output_get)
  (`self.SendData` ConnectionId (`self.Conv_StringToBytes` _output_get)))

(event `self.ReceiveTick`
  (params (DeltaSeconds :type "Float (single-precision)")))

(event `ReciveMsg`
  (params (ConnectionId :type Integer) (Message :type "Array of Byte (by ref)"))
  (bind _as_bp_first_person_character (`self.As BP First Person Character`))
  (bind _as_bp_first_person_character_2 (`self.As BP First Person Character`))
  (bind _as_bp_first_person_character_3 (`self.As BP First Person Character`))
  (bind _as_bp_first_person_character_4 (`self.As BP First Person Character`))
  (bind _returnvalue (`self.GetComponentByClass` _as_bp_first_person_character_2 "/Game/Blueprints_HS/BP_Weapon_Component.BP_Weapon_Component_C"))
  (bind _returnvalue_2 (`self.Message_ReadString` Message 25))
  (`KismetSystemLibrary.PrintString` _returnvalue_2)
  (`|ExecutionSequence`
    (:`then_0`
      (bind _returnvalue_3 (`KismetStringLibrary.ParseIntoArray` _returnvalue_2 "/"))
      (bind (_x _y) (`self.GetFianlXY` (`KismetStringLibrary.Conv_StringToDouble` (`|GetArrayItem` _returnvalue_3)) (`KismetStringLibrary.Conv_StringToDouble` (`|GetArrayItem` _returnvalue_3 1)) (`KismetStringLibrary.Conv_StringToDouble` (`|GetArrayItem` _returnvalue_3 2)) (`KismetStringLibrary.Conv_StringToDouble` (`|GetArrayItem` _returnvalue_3 3))))
      (bind (_resultx _resulty) (`self.CompensateXY` (`self.compensateVal`) _x _y))
      (`/Engine/EditorBlueprintResources/StandardMacros.IsValid` _as_bp_first_person_character
        (:`Is Valid`
          (`/Game/Blueprints_HS/BP_FirstPersonCharacter.MoveCamera` _as_bp_first_person_character (* _resultx -1.0) _resulty))
        (:`Is Not Valid`
          (`KismetSystemLibrary.PrintString` "ERROR!! : Player OBJ NULL"))))
    (:`then_1`
      (bind _returnvalue_4 (`KismetStringLibrary.Conv_StringToInt` (`|GetArrayItem` _returnvalue_3 4)))
      (if (or (== _returnvalue_4 1) (== _returnvalue_4 3))
        (`/Engine/EditorBlueprintResources/StandardMacros.IsValid` _as_bp_first_person_character_2
          (:`Is Valid`
            (`/Engine/EditorBlueprintResources/StandardMacros.IsValid` _returnvalue
              (:`Is Valid`
                (`/Game/Blueprints_HS/BP_Weapon_Component.Fire` _returnvalue))))
          (:`Is Not Valid`
            (`KismetSystemLibrary.PrintString` "ERROR!! : Player OBJ NULL")))))
    (:`then_2`
      (if (or (== _returnvalue_4 2) (== _returnvalue_4 3))
        (`/Engine/EditorBlueprintResources/StandardMacros.IsValid` _as_bp_first_person_character_3
          (:`Is Valid`
            (`/Game/Blueprints_HS/BP_FirstPersonCharacter.SetFlying` _as_bp_first_person_character_3))
          (:`Is Not Valid`
            (`KismetSystemLibrary.PrintString` "ERROR!! : Player OBJ NULL")))
        (else
          (`/Engine/EditorBlueprintResources/StandardMacros.IsValid` _as_bp_first_person_character_4
            (:`Is Valid`
              (if (`/Game/Blueprints_HS/BP_FirstPersonCharacter.bNowFlying` _as_bp_first_person_character_4)
                (`/Game/Blueprints_HS/BP_FirstPersonCharacter.SetFall` _as_bp_first_person_character_4)))
            (:`Is Not Valid`
              (`KismetSystemLibrary.PrintString` "ERROR!! : Player OBJ NULL"))))))))

(event `SetBool`
  (set `self.NowDelay` false))

(fn `CompensateXY`
  (params (compensateVal :type "Float (double-precision)") (x :type "Float (double-precision)") (y :type "Float (double-precision)"))
  (returns (ResultX :type "Float (double-precision)") (ResultY :type "Float (double-precision)"))
  (locals (RX :type "Float (double-precision)") (RY :type "Float (double-precision)"))
  (`|ExecutionSequence`
    (:`then_0`
      (if (< compensateVal (`KismetMathLibrary.Abs` x))
        (set `local.RX` x)
        (else
          (set `local.RX` 0.0))))
    (:`then_1`
      (if (< compensateVal (`KismetMathLibrary.Abs` y))
        (set `local.RY` y)
        (else
          (set `local.RY` 0.0))))
    (:`then_2`
      (return (`local.RX`) (`local.RY`)))))

(fn `GetFianlXY`
  (params (xp :type "Float (double-precision)") (xm :type "Float (double-precision)") (yp :type "Float (double-precision)") (ym :type "Float (double-precision)"))
  (returns (X :type "Float (double-precision)") (Y :type "Float (double-precision)"))
  (locals (`Result X` :type "Float (double-precision)") (`Result Y` :type "Float (double-precision)"))
  (`|ExecutionSequence`
    (:`then_0`
      (if (> xp 0.0)
        (set `local.Result X` xp)
        (else
          (set `local.Result X` (* xm -1.0)))))
    (:`then_1`
      (if (> yp 0.0)
        (set `local.Result Y` yp)
        (else
          (set `local.Result Y` (* ym -1.0)))))
    (:`then_2`
      (return (`local.Result X`) (`local.Result Y`)))))

(fn `UserConstructionScript`)