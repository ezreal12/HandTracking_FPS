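; BP_Enemy is an enemy character that shows its health as text and dies in an explosion when health runs out.
; DiscountHP subtracts damage, refreshes the HPRender text and calls Death at zero or below.
; Death spawns an explosion effect and sound at the actor's location, then destroys it.
; UpdateWalkSpeed lets callers change its maximum walk speed.
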(event `self.ReceiveBeginPlay`
  (`TextRenderComponent.K2_SetText` (`self.HPRender`) (`KismetTextLibrary.Conv_DoubleToText` (`self.HP`) "HalfToEven")))

(fn `Death`
  (bind _returnvalue (`self.K2_GetActorLocation`))
  (`GameplayStatics.SpawnEmitterAtLocation` "/Game/StarterContent/Particles/P_Explosion.P_Explosion" _returnvalue)
  (`GameplayStatics.PlaySoundAtLocation` "/Game/StarterContent/Audio/Explosion01.Explosion01" _returnvalue (struct) 1.0 1.0 0.0 null null null null)
  (`self.K2_DestroyActor`))

(fn `Discount HP`
  (params (Discount :type "Float (double-precision)" :default 20.0))
  (bind _output_get (set `self.HP` (- (`self.HP`) Discount)))
  (`TextRenderComponent.K2_SetText` (`self.HPRender`) (`KismetTextLibrary.Conv_DoubleToText` _output_get "HalfToEven"))
  (if (<= (`self.HP`) 0.0)
    (`self.Death`)))

(fn `UpdateWalkSpeed`
  (params (`Max Speed` :type "Float (double-precision)"))
  (set `CharacterMovementComponent.MaxWalkSpeed` `Max Speed` (`self.CharacterMovement`)))

(fn `UserConstructionScript`)